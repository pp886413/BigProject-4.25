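; Game instance Blueprint that restores the player's saved audio levels when the game starts.
; On Init, after the parent call, it checks for the "Audio" save slot, loads it as a ProjectSaveGame and copies the music, sound effect and UI levels into its own variables.
; It only stores these values and does not apply them to any sound mix or create a save when none exists.
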(event EventInit
  (|CallParentFunction)
  (bind _returnvalue (SaveGame|DoesSaveGameExist "Audio"))
  (if _returnvalue
    (bind _returnvalue_2 (SaveGame|LoadGamefromSlot "Audio"))
    (bind _asproject_save_game (Utilities|Casting|CastToProjectSaveGame _returnvalue_2))
    (Variables|Default|SetGameMusicMagnitude (Variables|/Game/GameSave/ProjectSaveGame.ProjectSaveGame_C|GetSavedGameMusic _asproject_save_game))
    (Variables|Default|SetGameSoundEffectMagnitude (Variables|/Game/GameSave/ProjectSaveGame.ProjectSaveGame_C|GetSavedGameSound _asproject_save_game))
    (Variables|Default|SetGameUIMagnitude (Variables|/Game/GameSave/ProjectSaveGame.ProjectSaveGame_C|GetSavedGameUiSound _asproject_save_game))))