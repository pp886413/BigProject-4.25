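; Base weapon Blueprint that holds damage, energy and combo data and handles melee hits on enemies.
; HitEnemy sphere-traces from DamagePoint, skipping enemies already hit, then applies damage, life steal or power gain, and effects.
; Bosses also get hit-part bone shake, and brief time dilation adds impact, with its own wait on combo index 3.
; The breakable-object branch is present but unconnected, so it never runs.
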(event EventBeginPlay
  (Default|ResetFadeValue(StaticMesh) (Variables|Default|GetMeshMaterialFadeComp)))

(fn ConstructionScript
  (Variables|Default|SetWeaponData (Utilities|Struct|MakeWeaponData 2e+01 15.0 5e+01 1.1 2.0 true)))

(fn HitEnemy
  (bind _damagepoint (Variables|Default|GetDamagePoint))
  (bind _returnvalue (Transformation|GetWorldLocation _damagepoint))
  ;[1 1 1 1 30] Sphere trace to detect is enemy or breakable object
  (bind (_outhit _returnvalue_2) (Collision|SphereTraceForObjects _returnvalue (+ _returnvalue (* (Math|Vector|GetUpVector (Variables|Default|GetDamagePoint)) 1e+02)) 2e+01 (Utilities|Array|MakeArray "ObjectTypeQuery3" "ObjectTypeQuery6") false (Utilities|Array|MakeArray (Game|Player|GetPlayerPawn 0)) "None" true "(R=1.000000,G=0.000000,B=0.000000,A=1.000000)" "(R=0.000000,G=1.000000,B=0.000000,A=1.000000)" 1.0))
  (if _returnvalue_2
    (Utilities|FlowControl|Sequence
      (:then_0
        (if (Actor|ActorHasTag (.HitActor (Collision|BreakHitResult _outhit)) "Enemy")
          (if (not (Utilities|Array|ContainsItem (Variables|Default|GetHittedEnemy) (.HitActor (Collision|BreakHitResult _outhit))))
            (bind _returnvalue_3 (Utilities|Array|Add (Variables|Default|GetHittedEnemy) (.HitActor (Collision|BreakHitResult _outhit))))
            (bind _asenemy_base (Utilities|Casting|CastToEnemy_Base (Utilities|Array|Get(acopy) (Variables|Default|GetHittedEnemy) _returnvalue_3)))
            (bind _output_get (LocalVariables|SetTempEnemy _asenemy_base))
            (bind _asplayer_bp (Utilities|Casting|CastToPlayer_Bp (Game|Player|GetPlayerPawn 0)))
            (bind _output_get_2 (LocalVariables|SetTempPlayer _asplayer_bp))
            ;[1 0.007074 0.05484 1 20] If is power mode , damage will deal life steal
            (if (Variables|/Game/player/Player_Bp.Player_Bp_C|GetIsPowerMode _output_get_2)
              (Default|LifeSteal (LocalVariables|GetTempPlayer))
              (else
                ;[1 1 1 1 20] Add player power value
                (Default|AddPowerValue (LocalVariables|GetTempPlayer))))
            (if (Actor|ActorHasTag _output_get "Boss")
              ;[1 1 1 1 30] Hit part bone shaking(Boss only)
              (Default|HitPartCheck (LocalVariables|GetTempEnemy) (Utilities|GetDisplayName (.PhysMat (Collision|BreakHitResult _outhit))))
              (Utilities|Time|SetTimerbyFunctionName (LocalVariables|GetTempEnemy) "BoneMoveRotation" 0.01 true))
            ;[1 1 1] Damage to enemy and set health
            (Default|SetEnemyHP (LocalVariables|GetTempEnemy) (.damage (Variables|Default|GetWeaponData)))
            ;[1 1 1 1 20] Set enemy under health bar
            (Default|SetEnemyUnderHp (LocalVariables|GetTempEnemy))
            ;[1 1 1 1 30] Spawn hit particle
            (Effects|SpawnEmitteratLocation "/Game/All_Particles/FXVarietyPack/Particles/P_ky_hit1.P_ky_hit1" (.ImpactPoint (Collision|BreakHitResult _outhit)) "0, 0, 0" "0.200000,0.200000,0.200000")
            (Audio|PlaySound2D "/Game/All_Sounds/PlayerSounds/Used/Hit_Cue.Hit_Cue" (Variables|/Script/BigProject.BigProjectGameInstance|GetGameSoundEffectMagnitude (Variables|/Game/player/Player_Bp.Player_Bp_C|GetMainGameInstance (LocalVariables|GetTempPlayer))) 1.0 0.0 0 0)
            ;[1 1 1 1 20] Camera shaking
            (Default|AttackShakeSetting (LocalVariables|GetTempPlayer))
            (if (== (Variables|/Game/player/Player_Bp.Player_Bp_C|GetComboIndex (LocalVariables|GetTempPlayer)) 3)
              ;[1 1 1 1 30] Slow time to increase attack feeling
              (Class|BigProjectFunctionLib|StartAttackHitTimeSlow self (LocalVariables|GetAttackHitTimeDilation) (LocalVariables|GetHardWaitTime))
              (else
                (Class|BigProjectFunctionLib|StartAttackHitTimeSlow self (LocalVariables|GetAttackHitTimeDilation) (LocalVariables|GetNormalWaitDuration))))))))))